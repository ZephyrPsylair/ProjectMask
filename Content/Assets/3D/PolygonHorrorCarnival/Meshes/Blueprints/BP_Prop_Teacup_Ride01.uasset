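; BP_Prop_Teacup_Ride01 is an animated teacup ride prop from the PolygonHorrorCarnival asset set.
; On BeginPlay, it binds six RotatingMovement components to the teapot, the platform and four teacup meshes, one component per part.
; Each part gets its own rotation through SetUpdatedComponent, so the graph needs no Tick or timeline logic.
; The construction script is empty.
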(event `self.ReceiveBeginPlay`
  (`MovementComponent.SetUpdatedComponent` (`self.RotatingMovement`) (`self.SM_Prop_Teacup_Ride_01_Teapot_01`))
  (`MovementComponent.SetUpdatedComponent` (`self.RotatingMovement1`) (`self.SM_Prop_Teacup_Ride_01_Platform_01`))
  (`MovementComponent.SetUpdatedComponent` (`self.RotatingMovement2`) (`self.SM_Prop_Teacup_Ride_01_Teacup_01`))
  (`MovementComponent.SetUpdatedComponent` (`self.RotatingMovement3`) (`self.SM_Prop_Teacup_Ride_01_Teacup_02`))
  (`MovementComponent.SetUpdatedComponent` (`self.RotatingMovement4`) (`self.SM_Prop_Teacup_Ride_01_Teacup_03`))
  (`MovementComponent.SetUpdatedComponent` (`self.RotatingMovement5`) (`self.SM_Prop_Teacup_Ride_01_Teacup_04`)))

(fn `UserConstructionScript`)