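; Weeping Angel enemy character that chases the player while unseen and freezes when rendered.
; Each tick checks whether MaskCharacter was recently rendered, using render visibility as a line-of-sight stand-in.
; When rendered it stops movement, velocity and animation; otherwise it paths to the player via SimpleMoveToLocation, with debug prints for both states.
; InitializeShake picks idle, walk or sprint camera shake from its own speed, but nothing here calls it.
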(event `self.ReceiveTick`
  (params (DeltaSeconds :type "Float (single-precision)"))
  (if (`PrimitiveComponent.WasRecentlyRendered` (`self.MaskCharacter`) 0.05)
    (if (`self.IsMoving`)
      (`Controller.StopMovement` (`self.GetController`))
      (set `self.IsMoving` false)
      (set `SkeletalMeshComponent.GlobalAnimRateScale` 0.0 (`self.Mesh`))
      (set `MovementComponent.Velocity` (0.0 0.0 0.0) (`self.CharacterMovement`))
      (`KismetSystemLibrary.PrintString` "Rendered"))
    (else
      (`AIBlueprintHelperLibrary.SimpleMoveToLocation` (`self.GetController`) (`self.K2_GetActorLocation` (`GameplayStatics.GetPlayerCharacter` 0)))
      (set `self.IsMoving` true)
      (set `SkeletalMeshComponent.GlobalAnimRateScale` 1.0 (`self.Mesh`))
      (`KismetSystemLibrary.PrintString` "Not Rendered"))))

(fn `InitializeShake`
  (if (and (> (`KismetMathLibrary.VSize` (`self.GetVelocity`)) 0.0) (`self.CanJump`))
    (if (< (`KismetMathLibrary.VSize` (`self.GetVelocity`)) 300.0)
      (`PlayerController.ClientStartCameraShake` :`self` (`GameplayStatics.GetPlayerController` 0) :`Shake` "/Game/Blueprints/Camera/CameraShake/BP_WalkShake.BP_WalkShake_C")
      (else
        (`PlayerController.ClientStartCameraShake` :`self` (`GameplayStatics.GetPlayerController` 0) :`Shake` "/Game/Blueprints/Camera/CameraShake/BP_SprintShake.BP_SprintShake_C")))
    (else
      (`PlayerController.ClientStartCameraShake` :`self` (`GameplayStatics.GetPlayerController` 0) :`Shake` "/Game/Blueprints/Camera/CameraShake/BP_IdleShake.BP_IdleShake_C"))))

(fn `UserConstructionScript`)