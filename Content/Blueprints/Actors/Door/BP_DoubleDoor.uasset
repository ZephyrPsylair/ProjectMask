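; BP_DoubleDoor is a two-leaf door actor that either swings under physics or opens automatically when its trigger is overlapped.
; BeginPlay applies the physics setting and, for non-physics doors, stores each leaf's closed yaw relative to the actor.
; Trigger overlaps switch target yaws between open and closed, and Tick eases both leaves toward them with RInterpTo.
; Locked doors skip both setup and movement.
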(event `self.ReceiveBeginPlay`
  (bind (_returnvalue_roll _returnvalue_pitch _returnvalue_yaw) (`KismetMathLibrary.BreakRotator` (`self.K2_GetActorRotation`)))
  (bind (_returnvalue_roll_2 _returnvalue_pitch_2 _returnvalue_yaw_2) (`KismetMathLibrary.BreakRotator` (`self.K2_GetActorRotation`)))
  (bind _physicateddoor (`self.PhysicatedDoor`))
  (bind (_returnvalue_roll_3 _returnvalue_pitch_3 _returnvalue_yaw_3) (`KismetMathLibrary.BreakRotator` (`SceneComponent.K2_GetComponentRotation` (`self.DoorRight`))))
  (bind (_returnvalue_roll_4 _returnvalue_pitch_4 _returnvalue_yaw_4) (`KismetMathLibrary.BreakRotator` (`SceneComponent.K2_GetComponentRotation` (`self.DoorLeft`))))
  (if (not (`self.Locked`))
    (`PrimitiveComponent.SetSimulatePhysics` (`self.DoorLeft`) _physicateddoor)
    (`PrimitiveComponent.SetSimulatePhysics` (`self.DoorRight`) _physicateddoor)
    (if (not _physicateddoor)
      (bind _output_get (set `self.LeftDoorClosedAngle` (- _returnvalue_yaw_4 _returnvalue_yaw_2)))
      (set `self.LeftDoorTargetAngle` _output_get)
      (bind _output_get_2 (set `self.RightDoorClosedAngle` (- _returnvalue_yaw_3 _returnvalue_yaw)))
      (set `self.RightDoorTargetAngle` _output_get_2))))

(event `self.ReceiveTick`
  (params (DeltaSeconds :type "Float (single-precision)"))
  (bind (_returnvalue_roll _returnvalue_pitch _returnvalue_yaw) (`KismetMathLibrary.BreakRotator` (`self.K2_GetActorRotation`)))
  (bind (_returnvalue_roll_2 _returnvalue_pitch_2 _returnvalue_yaw_2) (`KismetMathLibrary.BreakRotator` (`self.K2_GetActorRotation`)))
  (bind _doorright (`self.DoorRight`))
  (bind _doorleft (`self.DoorLeft`))
  (bind _returnvalue (`SceneComponent.K2_GetComponentRotation` _doorright))
  (bind _returnvalue_2 (`SceneComponent.K2_GetComponentRotation` _doorleft))
  (if (not (`self.Locked`))
    (if (not (`self.PhysicatedDoor`))
      (set `self.DeltaSeconds` DeltaSeconds)
      (`SceneComponent.K2_SetWorldRotation` _doorleft (`KismetMathLibrary.RInterpTo` _returnvalue_2 (`KismetMathLibrary.MakeRotator` (.roll _returnvalue_2) (.pitch _returnvalue_2) (+ (`self.LeftDoorTargetAngle`) _returnvalue_yaw_2)) (`self.DeltaSeconds`) (`self.DoorSpeed`)) true false)
      (`SceneComponent.K2_SetWorldRotation` _doorright (`KismetMathLibrary.RInterpTo` _returnvalue (`KismetMathLibrary.MakeRotator` (.roll _returnvalue) (.pitch _returnvalue) (+ (`self.RightDoorTargetAngle`) _returnvalue_yaw)) (`self.DeltaSeconds`) (`self.DoorSpeed`)) true false))))

(event `self.DoorTrigger.OnComponentBeginOverlap`
  (params (OverlappedComponent :type "PrimitiveComponent Object Reference") (OtherActor :type "Actor Object Reference") (OtherComp :type "PrimitiveComponent Object Reference") (OtherBodyIndex :type Integer) (bFromSweep :type Boolean) (SweepResult :type "HitResult Structure (by ref)"))
  (set `self.LeftDoorTargetAngle` (`self.LeftDoorOpenAngle`))
  (set `self.RightDoorTargetAngle` (`self.RightDoorOpenAngle`)))

(event `self.DoorTrigger.OnComponentEndOverlap`
  (params (OverlappedComponent :type "PrimitiveComponent Object Reference") (OtherActor :type "Actor Object Reference") (OtherComp :type "PrimitiveComponent Object Reference") (OtherBodyIndex :type Integer))
  (set `self.LeftDoorTargetAngle` (`self.LeftDoorClosedAngle`))
  (set `self.RightDoorTargetAngle` (`self.RightDoorClosedAngle`)))

(fn `UserConstructionScript`)