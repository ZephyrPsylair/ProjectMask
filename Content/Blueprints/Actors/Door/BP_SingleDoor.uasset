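; BP_SingleDoor is a single door actor that either runs as a physics object or opens automatically through a trigger volume.
; In non-physics mode, BeginPlay records the closed yaw relative to the actor, and DoorTrigger overlaps switch the target between open and closed angles without filtering the overlapping actor.
; Tick eases the door's world yaw toward that actor-relative target with RInterpTo at DoorSpeed.
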(event `self.ReceiveBeginPlay`
  (bind (_returnvalue_roll _returnvalue_pitch _returnvalue_yaw) (`KismetMathLibrary.BreakRotator` (`self.K2_GetActorRotation`)))
  (bind _physicateddoor (`self.PhysicatedDoor`))
  (bind (_returnvalue_roll_2 _returnvalue_pitch_2 _returnvalue_yaw_2) (`KismetMathLibrary.BreakRotator` (`SceneComponent.K2_GetComponentRotation` (`self.Door`))))
  (`PrimitiveComponent.SetSimulatePhysics` (`self.Door`) _physicateddoor)
  (if (not _physicateddoor)
    (bind _output_get (set `self.DoorClosedAngle` (- _returnvalue_yaw_2 _returnvalue_yaw)))
    (set `self.DoorTargetAngle` _output_get)))

(event `self.ReceiveTick`
  (params (DeltaSeconds :type "Float (single-precision)"))
  (bind (_returnvalue_roll _returnvalue_pitch _returnvalue_yaw) (`KismetMathLibrary.BreakRotator` (`self.K2_GetActorRotation`)))
  (bind _door (`self.Door`))
  (bind _returnvalue (`SceneComponent.K2_GetComponentRotation` _door))
  (if (not (`self.PhysicatedDoor`))
    (set `self.DeltaSeconds` DeltaSeconds)
    (`SceneComponent.K2_SetWorldRotation` _door (`KismetMathLibrary.RInterpTo` _returnvalue (`KismetMathLibrary.MakeRotator` (.roll _returnvalue) (.pitch _returnvalue) (+ (`self.DoorTargetAngle`) _returnvalue_yaw)) (`self.DeltaSeconds`) (`self.DoorSpeed`)) true false)))

(event `self.DoorTrigger.OnComponentBeginOverlap`
  (params (OverlappedComponent :type "PrimitiveComponent Object Reference") (OtherActor :type "Actor Object Reference") (OtherComp :type "PrimitiveComponent Object Reference") (OtherBodyIndex :type Integer) (bFromSweep :type Boolean) (SweepResult :type "HitResult Structure (by ref)"))
  (set `self.DoorTargetAngle` (`self.DoorOpenAngle`)))

(event `self.DoorTrigger.OnComponentEndOverlap`
  (params (OverlappedComponent :type "PrimitiveComponent Object Reference") (OtherActor :type "Actor Object Reference") (OtherComp :type "PrimitiveComponent Object Reference") (OtherBodyIndex :type Integer))
  (set `self.DoorTargetAngle` (`self.DoorClosedAngle`)))

(fn `UserConstructionScript`)