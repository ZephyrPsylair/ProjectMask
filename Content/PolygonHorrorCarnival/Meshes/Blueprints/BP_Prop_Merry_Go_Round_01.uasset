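; Animated merry-go-round prop for the horror carnival that runs on its own from BeginPlay.
; RotatingMovement components are bound at startup to the rotating wood floor and to each of ten overhead crank arms, so each part spins under its own component.
; Two timelines, HorsePart1 and Timeline_0, each drive the relative Z location of half of the twenty horses, moving them up and down in two separate groups.
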(event `self.ReceiveBeginPlay`
  (`|ExecutionSequence`
    (:`then_0`
      (`MovementComponent.SetUpdatedComponent` (`self.RotatingMovement`) (`self.SM_Prop_Merry_Go_Round_01_SM_Prop_Merry_Go_Round_01_Rotate_01_WoodFloor_01`))
      (`MovementComponent.SetUpdatedComponent` (`self.RotatingMovement6`) (`self.Arm_05_Crank_06`))
      (`MovementComponent.SetUpdatedComponent` (`self.RotatingMovement2`) (`self.Arm_05_Crank_02`))
      (`MovementComponent.SetUpdatedComponent` (`self.RotatingMovement3`) (`self.Arm_05_Crank_03`))
      (`MovementComponent.SetUpdatedComponent` (`self.RotatingMovement4`) (`self.Arm_05_Crank_04`))
      (`MovementComponent.SetUpdatedComponent` (`self.RotatingMovement5`) (`self.Arm_05_Crank_05`))
      (`MovementComponent.SetUpdatedComponent` (`self.RotatingMovement1`) (`self.Arm_05_Crank_01`))
      (`MovementComponent.SetUpdatedComponent` (`self.RotatingMovement7`) (`self.Arm_05_Crank_07`))
      (`MovementComponent.SetUpdatedComponent` (`self.RotatingMovement8`) (`self.Arm_05_Crank_08`))
      (`MovementComponent.SetUpdatedComponent` (`self.RotatingMovement9`) (`self.Arm_05_Crank_09`))
      (`MovementComponent.SetUpdatedComponent` (`self.RotatingMovement10`) (`self.Arm_05_Crank_010`)))
    (:`then_1`
      (bind (_direction _horesup_and_down_1) (`Timeline|Horse part 1`)
        (:`Update`
          (`SceneComponent.K2_SetRelativeLocation` (`self.Ride_02_Horse_03`) (`KismetMathLibrary.MakeVector` 0.0 0.0 _horesup_and_down_1) false false)
          (`SceneComponent.K2_SetRelativeLocation` (`self.Ride_02_Horse_07`) (`KismetMathLibrary.MakeVector` 0.0 0.0 _horesup_and_down_1) false false)
          (`SceneComponent.K2_SetRelativeLocation` (`self.Ride_01_Horse_07`) (`KismetMathLibrary.MakeVector` 0.0 0.0 _horesup_and_down_1) false false)
          (`SceneComponent.K2_SetRelativeLocation` (`self.Ride_02_Horse_05`) (`KismetMathLibrary.MakeVector` 0.0 0.0 _horesup_and_down_1) false false)
          (`SceneComponent.K2_SetRelativeLocation` (`self.Ride_01_Horse_05`) (`KismetMathLibrary.MakeVector` 0.0 0.0 _horesup_and_down_1) false false)
          (`SceneComponent.K2_SetRelativeLocation` (`self.Ride_02_Horse_08`) (`KismetMathLibrary.MakeVector` 0.0 0.0 _horesup_and_down_1) false false)
          (`SceneComponent.K2_SetRelativeLocation` (`self.Ride_01_Horse_03`) (`KismetMathLibrary.MakeVector` 0.0 0.0 _horesup_and_down_1) false false)
          (`SceneComponent.K2_SetRelativeLocation` (`self.Ride_02_Horse_01`) (`KismetMathLibrary.MakeVector` 0.0 0.0 _horesup_and_down_1) false false)
          (`SceneComponent.K2_SetRelativeLocation` (`self.Ride_01_Horse_01`) (`KismetMathLibrary.MakeVector` 0.0 0.0 _horesup_and_down_1) false false)
          (`SceneComponent.K2_SetRelativeLocation` (`self.Ride_02_Horse_09`) (`KismetMathLibrary.MakeVector` 0.0 0.0 _horesup_and_down_1) false false))))
    (:`then_2`
      (bind (_direction_2 _horesup_and_down_1_2) (`Timeline|Timeline_0`)
        (:`Update`
          (`SceneComponent.K2_SetRelativeLocation` (`self.Ride_01_Horse_04`) (`KismetMathLibrary.MakeVector` 0.0 0.0 _horesup_and_down_1_2) false false)
          (`SceneComponent.K2_SetRelativeLocation` (`self.Ride_01_Horse_08`) (`KismetMathLibrary.MakeVector` 0.0 0.0 _horesup_and_down_1_2) false false)
          (`SceneComponent.K2_SetRelativeLocation` (`self.Ride_02_Horse_06`) (`KismetMathLibrary.MakeVector` 0.0 0.0 _horesup_and_down_1_2) false false)
          (`SceneComponent.K2_SetRelativeLocation` (`self.Ride_01_Horse_06`) (`KismetMathLibrary.MakeVector` 0.0 0.0 _horesup_and_down_1_2) false false)
          (`SceneComponent.K2_SetRelativeLocation` (`self.Ride_02_Horse_04`) (`KismetMathLibrary.MakeVector` 0.0 0.0 _horesup_and_down_1_2) false false)
          (`SceneComponent.K2_SetRelativeLocation` (`self.Ride_01_Horse_09`) (`KismetMathLibrary.MakeVector` 0.0 0.0 _horesup_and_down_1_2) false false)
          (`SceneComponent.K2_SetRelativeLocation` (`self.Ride_02_Horse_02`) (`KismetMathLibrary.MakeVector` 0.0 0.0 _horesup_and_down_1_2) false false)
          (`SceneComponent.K2_SetRelativeLocation` (`self.Ride_01_Horse_02`) (`KismetMathLibrary.MakeVector` 0.0 0.0 _horesup_and_down_1_2) false false)
          (`SceneComponent.K2_SetRelativeLocation` (`self.Ride_02_Horse_10`) (`KismetMathLibrary.MakeVector` 0.0 0.0 _horesup_and_down_1_2) false false)
          (`SceneComponent.K2_SetRelativeLocation` (`self.Ride_01_Horse_10`) (`KismetMathLibrary.MakeVector` 0.0 0.0 _horesup_and_down_1_2) false false))))))

(fn `UserConstructionScript`)