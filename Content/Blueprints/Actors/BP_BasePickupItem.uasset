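; Base actor for a world item that the player character picks up by interacting with it.
; The construction script applies the configured static mesh to the item's mesh component.
; On Interact, it passes its held-item class, its own pickup class, mesh, socket offset and rotation to the character's PickupItem, then destroys itself.
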(event `/Game/Blueprints/Interfaces/BPI_Interact.Interact`
  (params (PlayerCharacter :type "/Game/Blueprints/Characters/BP_MaskCharacter Object Reference"))
  (`/Game/Blueprints/Characters/BP_MaskCharacter.PickupItem` PlayerCharacter (`self.HeldItem`) (`GameplayStatics.GetObjectClass` self) (`self.SocketOffset`) (`self.ItemStaticMesh`) (`self.ItemRotation`))
  (`self.K2_DestroyActor`))

(fn `UserConstructionScript`
  (`StaticMeshComponent.SetStaticMesh` (`self.ItemMesh`) (`self.ItemStaticMesh`)))