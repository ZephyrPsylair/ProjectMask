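; BP_Prop_Ferris_Wheel_01 is an animated carnival Ferris wheel prop that starts moving on BeginPlay.
; Five RotatingMovement components are assigned to the main rotating mesh and four gear meshes to spin them.
; The Bench_Turn timeline sets the world rotation of all twelve seats from one shared track, swinging their pitch back and forth while keeping the root's yaw, so they do not tip with the wheel.
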(event `self.ReceiveBeginPlay`
  (bind (_returnvalue_roll _returnvalue_pitch _returnvalue_yaw) (`KismetMathLibrary.BreakRotator` (`SceneComponent.K2_GetComponentRotation` (`self.DefaultSceneRoot`))))
  (`|ExecutionSequence`
    (:`then_0`
      ;[1 1 1] Wheel rotation and break rotation
      (`MovementComponent.SetUpdatedComponent` (`self.RotatingMovement`) (`self.SM_Prop_Ferris_Wheel_01_Rotate_01`))
      (`MovementComponent.SetUpdatedComponent` (`self.RotatingMovement1`) (`self.SM_Prop_Ferris_Wheel_01_WheelGear_02`))
      (`MovementComponent.SetUpdatedComponent` (`self.RotatingMovement2`) (`self.SM_Prop_Ferris_Wheel_01_WheelGear_01`))
      (`MovementComponent.SetUpdatedComponent` (`self.RotatingMovement3`) (`self.SM_Prop_Ferris_Wheel_01_WheelGear_03`))
      (`MovementComponent.SetUpdatedComponent` (`self.RotatingMovement4`) (`self.SM_Prop_Ferris_Wheel_01_WheelGear_04`)))
    (:`then_1`
      ;[1 1 1] Chair swinging and potition
      (bind (_direction _bench_05) (`Timeline|Bench_Turn`)
        (:`Update`
          (`SceneComponent.K2_SetWorldRotation` (`self.SM_Prop_Ferris_Wheel_01_Seat_05`) (`KismetMathLibrary.RLerp` (`KismetMathLibrary.MakeRotator` 0.0 -20.0 _returnvalue_yaw) (`KismetMathLibrary.MakeRotator` 0.0 20.0 _returnvalue_yaw) _bench_05) false false)
          (`SceneComponent.K2_SetWorldRotation` (`self.SM_Prop_Ferris_Wheel_01_Seat_02`) (`KismetMathLibrary.RLerp` (`KismetMathLibrary.MakeRotator` 0.0 -20.0 _returnvalue_yaw) (`KismetMathLibrary.MakeRotator` 0.0 20.0 _returnvalue_yaw) _bench_05) false false)
          (`SceneComponent.K2_SetWorldRotation` (`self.SM_Prop_Ferris_Wheel_01_Seat_06`) (`KismetMathLibrary.RLerp` (`KismetMathLibrary.MakeRotator` 0.0 -20.0 _returnvalue_yaw) (`KismetMathLibrary.MakeRotator` 0.0 20.0 _returnvalue_yaw) _bench_05) false false)
          (`SceneComponent.K2_SetWorldRotation` (`self.SM_Prop_Ferris_Wheel_01_Seat_04`) (`KismetMathLibrary.RLerp` (`KismetMathLibrary.MakeRotator` 0.0 -20.0 _returnvalue_yaw) (`KismetMathLibrary.MakeRotator` 0.0 20.0 _returnvalue_yaw) _bench_05) false false)
          (`SceneComponent.K2_SetWorldRotation` (`self.SM_Prop_Ferris_Wheel_01_Seat_11`) (`KismetMathLibrary.RLerp` (`KismetMathLibrary.MakeRotator` 0.0 -20.0 _returnvalue_yaw) (`KismetMathLibrary.MakeRotator` 0.0 20.0 _returnvalue_yaw) _bench_05) false false)
          (`SceneComponent.K2_SetWorldRotation` (`self.SM_Prop_Ferris_Wheel_01_Seat_12`) (`KismetMathLibrary.RLerp` (`KismetMathLibrary.MakeRotator` 0.0 -20.0 _returnvalue_yaw) (`KismetMathLibrary.MakeRotator` 0.0 20.0 _returnvalue_yaw) _bench_05) false false)
          (`SceneComponent.K2_SetWorldRotation` (`self.SM_Prop_Ferris_Wheel_01_Seat_01`) (`KismetMathLibrary.RLerp` (`KismetMathLibrary.MakeRotator` 0.0 -20.0 _returnvalue_yaw) (`KismetMathLibrary.MakeRotator` 0.0 20.0 _returnvalue_yaw) _bench_05) false false)
          (`SceneComponent.K2_SetWorldRotation` (`self.SM_Prop_Ferris_Wheel_01_Seat_03`) (`KismetMathLibrary.RLerp` (`KismetMathLibrary.MakeRotator` 0.0 -20.0 _returnvalue_yaw) (`KismetMathLibrary.MakeRotator` 0.0 20.0 _returnvalue_yaw) _bench_05) false false)
          (`SceneComponent.K2_SetWorldRotation` (`self.SM_Prop_Ferris_Wheel_01_Seat_07`) (`KismetMathLibrary.RLerp` (`KismetMathLibrary.MakeRotator` 0.0 -20.0 _returnvalue_yaw) (`KismetMathLibrary.MakeRotator` 0.0 20.0 _returnvalue_yaw) _bench_05) false false)
          (`SceneComponent.K2_SetWorldRotation` (`self.SM_Prop_Ferris_Wheel_01_Seat_08`) (`KismetMathLibrary.RLerp` (`KismetMathLibrary.MakeRotator` 0.0 -20.0 _returnvalue_yaw) (`KismetMathLibrary.MakeRotator` 0.0 20.0 _returnvalue_yaw) _bench_05) false false)
          (`SceneComponent.K2_SetWorldRotation` (`self.SM_Prop_Ferris_Wheel_01_Seat_09`) (`KismetMathLibrary.RLerp` (`KismetMathLibrary.MakeRotator` 0.0 -20.0 _returnvalue_yaw) (`KismetMathLibrary.MakeRotator` 0.0 20.0 _returnvalue_yaw) _bench_05) false false)
          (`SceneComponent.K2_SetWorldRotation` (`self.SM_Prop_Ferris_Wheel_01_Seat_10`) (`KismetMathLibrary.RLerp` (`KismetMathLibrary.MakeRotator` 0.0 -20.0 _returnvalue_yaw) (`KismetMathLibrary.MakeRotator` 0.0 20.0 _returnvalue_yaw) _bench_05) false false))))))

(fn `UserConstructionScript`)