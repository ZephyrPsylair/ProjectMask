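; BP_DoubleDoorSystem is a two-leaf door that opens by enabling physics simulation on both leaves when unlocked through Interact.
; While locked, its trigger shows BP_MaskCharacter a message based on whether a held item has the "Key" tag, removing it on exit or interaction.
; Interact itself checks only PermanentLock, which also disables trigger overlaps and switches the construction-time actor tag from "Door" to "Not A Door".
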(event `self.ReceiveBeginPlay`
  (bind _doortrigger (`self.DoorTrigger`))
  (`PrimitiveComponent.SetSimulatePhysics` (`self.DoorLeft`) (`self.PhysicatedDoor`))
  (`PrimitiveComponent.SetSimulatePhysics` (`self.DoorRight`) (`self.PhysicatedDoor`))
  (if (`self.PermanentLock`)
    (set `PrimitiveComponent.bGenerateOverlapEvents` false _doortrigger)
    (else
      (set `PrimitiveComponent.bGenerateOverlapEvents` true _doortrigger))))

(event `self.DoorTrigger.OnComponentBeginOverlap`
  (params (OverlappedComponent :type "PrimitiveComponent Object Reference") (OtherActor :type "Actor Object Reference") (OtherComp :type "PrimitiveComponent Object Reference") (OtherBodyIndex :type Integer) (bFromSweep :type Boolean) (SweepResult :type "HitResult Structure (by ref)"))
  (bind _interacttext (`/Game/Blueprints/Widget/WBP_Message.InteractText` (`self.MessageWidget`)))
  (bind _asbp_mask_character (cast `/Game/Blueprints/Characters/BP_MaskCharacter` OtherActor))
  (`|ExecutionSequence`
    (:`then_0`
      (if (`self.IsLocked`)
        (`/Engine/EditorBlueprintResources/StandardMacros.DoOnce` false :!label _label
          (:`Completed`
            (bind _returnvalue (`|CreateWidget` "/Game/Blueprints/Widget/WBP_Message.WBP_Message_C"))
            (bind _output_get (set `self.MessageWidget` _returnvalue))
            (`UserWidget.AddToViewport` _output_get 0)
            (bind _holdingitem (`/Game/Blueprints/Characters/BP_MaskCharacter.HoldingItem` _asbp_mask_character))
            (if (and (`/Game/Blueprints/Characters/BP_MaskCharacter.IsHoldingItem` _asbp_mask_character) (`KismetSystemLibrary.IsValid` _holdingitem))
              (if (`self.ActorHasTag` _holdingitem "Key")
                (set `TextBlock.Text` "Press E to Open" _interacttext)
                (else
                  (set `TextBlock.Text` "Locked" _interacttext :!label _label_2)))
              (else
                (goto _label_2)))
            (`/Game/Blueprints/Widget/WBP_Message.ToggleMessageVisiblity` (`self.MessageWidget`) true)))))
    (:`then_1`
      (goto _label_3 :!via `Reset`))))

(event `self.DoorTrigger.OnComponentEndOverlap`
  (params (OverlappedComponent :type "PrimitiveComponent Object Reference") (OtherActor :type "Actor Object Reference") (OtherComp :type "PrimitiveComponent Object Reference") (OtherBodyIndex :type Integer))
  (cast `/Game/Blueprints/Characters/BP_MaskCharacter` OtherActor)
  (`/Engine/EditorBlueprintResources/StandardMacros.DoOnce` false :!label _label_3
    (:`Completed`
      (bind _messagewidget (`self.MessageWidget`)
        (:`then`
          (`/Game/Blueprints/Widget/WBP_Message.ToggleMessageVisiblity` _messagewidget false)
          (`KismetSystemLibrary.Delay` 0.15)
          (`Widget.RemoveFromParent` _messagewidget)
          (goto _label :!via `Reset`))
        (:`else`)))))

(event `/Game/Blueprints/Interfaces/BPI_Interact.Interact`
  (params (PlayerCharacter :type "/Game/Blueprints/Characters/BP_MaskCharacter Object Reference"))
  (if (not (`self.PermanentLock`))
    (set `self.IsLocked` false)
    (bind _output_get (set `self.PhysicatedDoor` true))
    (`PrimitiveComponent.SetSimulatePhysics` (`self.DoorLeft`) _output_get)
    (`PrimitiveComponent.SetSimulatePhysics` (`self.DoorRight`) _output_get)
    (`/Engine/EditorBlueprintResources/StandardMacros.DoOnce` false
      (:`Completed`
        (bind _messagewidget (`self.MessageWidget`)
          (:`then`
            (`/Game/Blueprints/Widget/WBP_Message.ToggleMessageVisiblity` _messagewidget false)
            (`KismetSystemLibrary.Delay` 0.15)
            (`Widget.RemoveFromParent` _messagewidget))
          (:`else`))))))

(fn `UserConstructionScript`
  (if (`self.PermanentLock`)
    (set `self.Tags` (`|MakeArray` "Not A Door" :!type "Name"))
    (else
      (set `self.Tags` (`|MakeArray` "Door" :!type "Name")))))