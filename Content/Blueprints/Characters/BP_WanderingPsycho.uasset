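; BP_WanderingPsycho is an enemy character that roams random nearby reachable points, pausing between moves.
; When PawnSensing sees a pawn, it chases the first player and attacks on arrival, resuming roaming once a retriggerable delay lapses without sightings.
; Attack plays a montage, using a DoOnce and CanAttack flag to block repeats for its duration.
; InitializeShake, uncalled here, picks idle, walk or sprint camera shakes from its own velocity.
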(event `self.ReceiveBeginPlay`
  (`self.RandomRoam`))

(event `RandomRoam`
  (`|AIMoveTo` self (`NavigationSystemV1.K2_GetRandomReachablePointInRadius` (`self.K2_GetActorLocation`) 1500.0 null null) null
    (:`OnSuccess`
      (`KismetSystemLibrary.Delay` 2.0)
      (`self.RandomRoam`))))

(event `self.PawnSensing.OnSeePawn`
  (params (Pawn :type "Pawn Object Reference"))
  (set `self.CanAttack` true)
  (`|ExecutionSequence`
    (:`then_0`
      (`|AIMoveTo` self (0.0 0.0 0.0) (`GameplayStatics.GetPlayerCharacter` 0) 10.0
        (:`OnSuccess`
          (if (`self.CanAttack`)
            (set `self.CanAttack` false)
            (`self.Attack`)))))
    (:`then_1`
      (`KismetSystemLibrary.RetriggerableDelay` 1.0)
      (`self.RandomRoam`))))

(event `Attack`
  (`/Engine/EditorBlueprintResources/StandardMacros.DoOnce` false :!label _label
    (:`Completed`
      (bind _returnvalue (`self.PlayAnimMontage` "/Game/Assets/Animations/UE4/Movement/AM_Attack.AM_Attack"))
      (`KismetSystemLibrary.Delay` _returnvalue)
      (set `self.CanAttack` true)
      (goto _label :!via `Reset`))))

(fn `InitializeShake`
  (if (and (> (`KismetMathLibrary.VSize` (`self.GetVelocity`)) 0.0) (`self.CanJump`))
    (if (< (`KismetMathLibrary.VSize` (`self.GetVelocity`)) 300.0)
      (`PlayerController.ClientStartCameraShake` :`self` (`GameplayStatics.GetPlayerController` 0) :`Shake` "/Game/Blueprints/Camera/CameraShake/BP_WalkShake.BP_WalkShake_C")
      (else
        (`PlayerController.ClientStartCameraShake` :`self` (`GameplayStatics.GetPlayerController` 0) :`Shake` "/Game/Blueprints/Camera/CameraShake/BP_SprintShake.BP_SprintShake_C")))
    (else
      (`PlayerController.ClientStartCameraShake` :`self` (`GameplayStatics.GetPlayerController` 0) :`Shake` "/Game/Blueprints/Camera/CameraShake/BP_IdleShake.BP_IdleShake_C"))))

(fn `UserConstructionScript`)